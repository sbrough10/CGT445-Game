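; MinionCharacter is an AI minion character that fires projectiles and can be killed.
; StartFiring runs a looping timer at an interval of one over RateOfFire, spawning a MinionProjectile at ProjectileSpawnPoint each time until StopFiring clears it.
; AffectHealth adds a signed delta to Health through CalculateHealth, which updates IsDead, then prints Health for debugging and destroys the actor once dead.
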(event Custom|StartFiring
  ;[1 1 1] Shoot Projectile
  (Utilities|Time|SetTimerbyFunctionName 0 "FireWeapon" (/ 1.0 (Variables|Default|GetRateOfFire)) true))

(event Custom|StopFiring
  ;[1 1 1] Shoot Projectile
  (Utilities|Time|ClearTimerbyFunctionName 0 "FireWeapon"))

(event Custom|FireWeapon
  ;[1 1 1] Shoot Projectile
  (Game|SpawnActorfromClass "/Game/Blueprints/AI/MinionProjectile.MinionProjectile_C" (Transformation|GetWorldTransform (Variables|Default|GetProjectileSpawnPoint)) "Undefined" 0 0))

(event EventBeginPlay)

(event Collision|EventActorBeginOverlap
  (params (OtherActor :type Actor%20Object%20Reference)))

(event EventTick
  (params (DeltaSeconds :type Float%20%28single-precision%29)))

(event EventAffectHealth
  (params (Delta :type Float%20%28single-precision%29))
  (CallFunction|CalculateHealth Delta)
  (Development|PrintString (Utilities|String|ToString(Float) (Variables|Default|GetHealth)))
  (if (Variables|Default|GetisDead?)
    (Actor|DestroyActor)))

(fn ConstructionScript)

(fn CalculateDead
  (if (<= (Variables|Default|GetHealth) 0.0)
    (Variables|Default|SetisDead? true)
    (else
      (Variables|Default|SetisDead? false))))

(fn CalculateHealth
  (params (Delta :type Float%20%28single-precision%29))
  (Variables|Default|SetHealth (+ Delta (Variables|Default|GetHealth)))
  (CallFunction|CalculateDead))