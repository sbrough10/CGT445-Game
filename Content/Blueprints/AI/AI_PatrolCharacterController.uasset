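; AI controller for minion characters that patrol and attack the player on sight.
; On possessing a MinionCharacter it runs the Patrol_BT behavior tree.
; AI perception updates for the player write the sensed state to the CanSeePlayer? blackboard key and start or stop the minion's firing directly from the controller.
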(event OnTargetPerceptionUpdated(AIPerception)
  (params (Actor :type Actor%20Object%20Reference) (Stimulus :type AI%20Stimulus%20Structure))
  (bind _bsuccessfullysensed (Utilities|Struct|BreakAIStimulus Stimulus))
  (bind _returnvalue (Pawn|GetControlledPawn))
  (Utilities|Casting|CastToPlayerBP Actor)
  (AI|Components|Blackboard|SetValueasBool (AI|GetBlackboard 0) (Utilities|Name|MakeLiteralName "CanSeePlayer?") _bsuccessfullysensed)
  (if _bsuccessfullysensed
    (bind _asminion_character (Utilities|Casting|CastToMinionCharacter _returnvalue))
    (Default|StartFiring _asminion_character)
    (else
      (bind _asminion_character_2 (Utilities|Casting|CastToMinionCharacter _returnvalue))
      (Default|StopFiring _asminion_character_2))))

(event EventBeginPlay)

(event EventTick
  (params (DeltaSeconds :type Float%20%28single-precision%29)))

(event EventOnPossess
  (params (PossessedPawn :type Pawn%20Object%20Reference))
  (Utilities|Casting|CastToMinionCharacter PossessedPawn)
  (AI|RunBehaviorTree "/Game/Blueprints/AI/Patrol_BT.Patrol_BT"))

(fn ConstructionScript)