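; Paper2D player character for a side-scroller: a bird that walks, flaps, pecks goblins and shouts projectiles.
; InputEvent sets movement and action flags, which Tick turns into movement and delay-locked flipbook animations.
; Air flaps and shouts spend energy that refills each tick on the HUD bar.
; Hit updates taco health, flags knockback and shows Game Over at zero; its directional launch logic is disconnected.
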(event OnComponentBeginOverlap(PeckRange)
  (params (OverlappedComponent :type Primitive%20Component%20Object%20Reference) (OtherActor :type Actor%20Object%20Reference) (OtherComp :type Primitive%20Component%20Object%20Reference) (OtherBodyIndex :type Integer) (bFromSweep :type Boolean) (SweepResult :type Hit%20Result%20Structure%20%28by%20ref%29))
  (bind _asbpgoblin (Utilities|Casting|CastToBPGoblin OtherActor))
  (if (Variables|Default|GetIs%20Pecking)
    (Default|Damage _asbpgoblin 25 "NewEnumerator0")))

(event EventBeginPlay
  (Variables|Default|SetHealth 1.0))

(event EventTick
  (params (DeltaSeconds :type Float%20%28single-precision%29))
  (bind _hud_ui (Variables|Default|GetHUD%20UI))
  (bind _energybarfill (Variables|/Game/Blueprints/HUD.HUD_C|GetEnergyBarFill _hud_ui))
  (bind _rendertransform (Variables|/Script/UMG.Widget|GetRenderTransform _energybarfill))
  (bind _scale (Utilities|Struct|BreakWidgetTransform _rendertransform))
  (bind _returnvalue (+ _scale "(X=0.005000,Y=0.000000)"))
  (bind _x (Math|Vector2D|BreakVector2D _returnvalue))
  (if (not (Variables|Default|GetIs%20Knocked%20Back))
    (Pawn|Input|AddMovementInput "0.500000,0.000000, 0" (Variables|Default|GetHorizontal%20Movement) false))
  (if (< (- (Variables|Default|GetUpdate%20Animation%20Delay) DeltaSeconds) 0.0)
    (Variables|Default|SetUpdate%20Animation%20Delay 0.0)
    (else
      (Variables|Default|SetUpdate%20Animation%20Delay (- (Variables|Default|GetUpdate%20Animation%20Delay) DeltaSeconds))))
  (CallFunction|UpdateAnimation)
  (if (<= _x 1.0)
    (Widget|Transform|SetRenderScale _energybarfill _returnvalue)
    (Variables|Default|SetEnergy%20Level _x)))

(fn ConstructionScript
  (Variables|Default|SetHealth 1e+02))

(fn Hit
  (params (Damage :type Float%20%28single-precision%29) (Direction :type Direction%20Enum))
  (bind _output_get (Variables|Default|SetHealth (- (Variables|Default|GetHealth) Damage)))
  (Default|UpdateHealthTacos (Variables|Default|GetHUD%20UI) _output_get)
  (Variables|Default|SetIs%20Knocked%20Back true)
  (if (<= _output_get 0.0)
    (bind _returnvalue (UserInterface|CreateWidget "/Game/Blueprints/GameOver.GameOver_C"))
    (UserInterface|Viewport|AddtoViewport _returnvalue 0)
    (Game|SetGamePaused true)))

(fn UpdateAnimation
  (bind _sprite (Variables|Default|GetSprite))
  (bind _returnvalue (Class|PaperFlipbookComponent|GetFlipbookLength _sprite))
  (if (<= (Variables|Default|GetUpdate%20Animation%20Delay) 0.0)
    (if (Variables|Default|GetIs%20Knocked%20Back)
      (Variables|Default|SetIs%20Knocked%20Back false)
      (Sprite|SetFlipbook _sprite "/Game/Assets/Animations/Player/Standing.Standing" :!label _label)
      (elif (Variables|Default|GetIs%20Pecking)
        (Sprite|SetFlipbook _sprite "/Game/Assets/Animations/Player/Attack.Attack")
        (Variables|Default|SetUpdate%20Animation%20Delay _returnvalue)
        (Variables|Default|SetIs%20Pecking false)
        (elif (Variables|Default|GetJust%20Jumped)
          (Sprite|SetFlipbook _sprite "/Game/Assets/Animations/Player/FlapWings.FlapWings")
          (Variables|Default|SetUpdate%20Animation%20Delay _returnvalue)
          (Variables|Default|SetJust%20Jumped false)
          (elif (AI|Components|NavMovement|IsMovingonGround (Variables|Character|GetCharacterMovement))
            (if (Variables|Default|GetIs%20Moving)
              (Sprite|SetFlipbook _sprite "/Game/Assets/Animations/Player/Walking.Walking")
              (else
                (goto _label)))
            (else
              (Sprite|SetFlipbook _sprite "/Game/Assets/Animations/Player/Jumping.Jumping"))))))))

(fn InputEvent
  (params (Key :type Key%20Structure :default "AnyKey") (Pressed :type Boolean))
  (bind _walk_left_key (Variables|Default|GetWalk%20Left%20Key))
  (bind _walk_right_key (Variables|Default|GetWalk%20Right%20Key))
  (bind _camera (Variables|Default|GetCamera))
  (bind _sprite (Variables|Default|GetSprite))
  (bind _returnvalue (== Key _walk_right_key))
  (bind _returnvalue_2 (== Key _walk_left_key))
  (if (not (Variables|Default|GetIs%20Knocked%20Back))
    (if Pressed
      (if (== Key (Variables|Default|GetJump%20Key))
        (if (AI|Components|NavMovement|IsMovingonGround (Variables|Character|GetCharacterMovement))
          (Character|LaunchCharacter "0, 0,400.000000" false true)
          (Variables|Default|SetJust%20Jumped true :!label _label)
          (else
            (bind _has_sufficient_energy (CallFunction|DepleteEnergy 0.1))
            (if _has_sufficient_energy
              (Character|LaunchCharacter "0, 0,200.000000" false false)
              (goto _label))))
        (elif (== Key (Variables|Default|GetPeck%20Key))
          (Variables|Default|SetIs%20Pecking true)
          (elif _returnvalue_2
            (Variables|Default|SetHorizontal%20Movement -1.0)
            (Transformation|SetRelativeRotation _sprite "0,180.000000, 0" false false)
            (Variables|Default|SetIs%20Moving true :!label _label_2)
            (elif _returnvalue
              (Variables|Default|SetHorizontal%20Movement 1.0)
              (Transformation|SetRelativeRotation _sprite "0,0.000000, 0" false false)
              (goto _label_2)
              (elif (== Key (Variables|Default|GetShout%20Key))
                (bind _has_sufficient_energy_2 (CallFunction|DepleteEnergy 0.75))
                (if _has_sufficient_energy_2
                  (Game|SpawnActorfromClass "/Game/Blueprints/ArrowBP.ArrowBP_C" (Transformation|GetWorldTransform (Variables|Default|GetShoutSpawn)) "AlwaysSpawn" 0 0.0 0))
                (elif (== Key (Variables|Default|GetThrow%20Image%20Key))
                  (Transformation|SetRelativeLocation _camera (+ (Variables|/Script/Engine.SceneComponent|GetRelativeLocation _camera) "0.000000,200.000000,0.000000") false false)))))))
      (elif (or _returnvalue_2 _returnvalue)
        (Variables|Default|SetHorizontal%20Movement 0.0)
        (Variables|Default|SetIs%20Moving false)))))

(fn DepleteEnergy
  (params (Amount :type Float%20%28single-precision%29))
  (if (>= (- (Variables|Default|GetEnergy%20Level) Amount) 0.0)
    (Widget|Transform|SetRenderScale (Variables|/Game/Blueprints/HUD.HUD_C|GetEnergyBarFill (Variables|Default|GetHUD%20UI)) (Math|Vector2D|MakeVector2D (- (Variables|Default|GetEnergy%20Level) Amount) 1.0))
    (Variables|Default|SetEnergy%20Level (- (Variables|Default|GetEnergy%20Level) Amount)))
  (return (>= (- (Variables|Default|GetEnergy%20Level) Amount) 0.0)))