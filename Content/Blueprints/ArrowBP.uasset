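; ArrowBP is an arrow projectile whose launch speed comes from its Speed variable, applied to the projectile movement in the construction script.
; Hitting a PlayerBP deals a small fixed damage with a fixed direction and destroys the arrow at once.
; Any other hit plays a Wobble timeline that rotates the arrow slightly, disables its collision and destroys it after a short delay.
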(event Collision|EventHit
  (params (MyComp :type Primitive%20Component%20Object%20Reference) (Other :type Actor%20Object%20Reference) (OtherComp :type Primitive%20Component%20Object%20Reference) (bSelfMoved :type Boolean) (HitLocation :type Vector :default "0, 0, 0") (HitNormal :type Vector :default "0, 0, 0") (NormalImpulse :type Vector :default "0, 0, 0") (Hit :type Hit%20Result%20Structure%20%28by%20ref%29))
  (bind _asplayer_bp (Utilities|Casting|CastToPlayerBP Other)
    (:then
      (Default|Hit _asplayer_bp 0.1 "NewEnumerator0")
      (Actor|DestroyActor))
    (:CastFailed
      (bind _wobble (Timeline|Wobble Play)
        (:Update
          (Transformation|SetRelativeRotation (Variables|Default|GetScene) (Math|Rotator|Lerp(Rotator) "0, 0, 0" "10.000000, 0, 0" _wobble) false false)
          (Collision|SetCollisionEnabled (Variables|Default|GetCollision) "NoCollision")
          (Utilities|FlowControl|Delay 3.0)
          (Actor|DestroyActor))))))

(fn ConstructionScript
  (Variables|/Script/Engine.ProjectileMovementComponent|SetInitialSpeed (Variables|Default|GetProjectileMovement) (Variables|Default|GetSpeed)))