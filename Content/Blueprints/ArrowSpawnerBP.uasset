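; ArrowSpawnerBP is an arrow-launcher actor that moves while it repeatedly spawns ArrowBP actors.
; On BeginPlay it stores its start location, starts a looping half-second timer that spawns an arrow at the SpawnPoint transform with a fixed speed, and plays the Movement timeline.
; The timeline lerps the actor from its start location toward that location offset by the Speed vector, which acts as a displacement.
; A pitch-increment rotation node is left unconnected.
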(event Custom|fire
  (Game|SpawnActorfromClass "/Game/Blueprints/ArrowBP.ArrowBP_C" (Transformation|GetWorldTransform (Variables|Default|GetSpawnPoint)) "AlwaysSpawn" 0 4e+02 0))

(event EventBeginPlay
  (bind _speed (Variables|Default|GetSpeed))
  (Variables|Default|SetStartPosition (Transformation|GetActorLocation))
  (Utilities|Time|SetTimerbyFunctionName 0 "fire" 0.5 true)
  (bind _move (Timeline|Movement PlayFromStart)
    (:Update
      (Transformation|SetActorLocation (Math|Vector|Lerp(Vector) (Variables|Default|GetStartPosition) (Math|Vector|MakeVector (+ (.x (Variables|Default|GetStartPosition)) (.x _speed)) (+ (.y (Variables|Default|GetStartPosition)) (.y _speed)) (+ (.z (Variables|Default|GetStartPosition)) (.z _speed))) _move) false false))))

(fn ConstructionScript)