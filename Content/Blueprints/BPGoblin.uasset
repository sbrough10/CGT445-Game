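; BPGoblin is a Paper2D goblin enemy that hurts the player on contact.
; A Damage event subtracts from EnemyHealth and destroys the goblin at zero or below.
; Capsule overlap casts to PlayerBP and calls Hit with fixed damage and direction.
; An unconnected timeline holds patrol logic between PointA and PointB with X-scale flipping at the ends, but never runs.
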(event OnComponentBeginOverlap(Capsule)
  (params (OverlappedComponent :type Primitive%20Component%20Object%20Reference) (OtherActor :type Actor%20Object%20Reference) (OtherComp :type Primitive%20Component%20Object%20Reference) (OtherBodyIndex :type Integer) (bFromSweep :type Boolean) (SweepResult :type Hit%20Result%20Structure%20%28by%20ref%29))
  (bind _asplayer_bp (Utilities|Casting|CastToPlayerBP OtherActor))
  (Default|Hit _asplayer_bp 0.1 "NewEnumerator0"))

(event Custom|Damage
  (params (DamageInt :type Integer) (Direction :type Direction%20Enum))
  ;[1 1 1] take damage
  (bind _output_get (Variables|Default|SetEnemyHealth (- (Variables|Default|GetEnemyHealth) DamageInt)))
  (if (<= _output_get 0)
    (Actor|DestroyActor)))

(fn ConstructionScript
  (bind _returnvalue (Transformation|GetActorLocation))
  (Transformation|SetActorLocation (Math|Vector|MakeVector (.x _returnvalue) (.y _returnvalue) (.z _returnvalue)) false false))