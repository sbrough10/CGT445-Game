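; Game controller that sets up the HUD and applies pickup effects to the player.
; On BeginPlay it adds the HUD widget to the viewport and caches the player pawn as otherPlayerBP.
; OnPickUp tells pickup types apart by casting: a mushroom calls the player's ScaleControl, while a ring increments RingsCollected.
; Each pickup also prints a colored on-screen message.
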(event EventBeginPlay
  (bind _returnvalue (UserInterface|CreateWidget "/Game/blueprint/HUD.HUD_C"))
  (bind _output_get (Variables|Default|SetHUDReference _returnvalue))
  (UserInterface|Viewport|AddtoViewport _output_get 0)
  (bind _asother_player_bp (Utilities|Casting|CastTootherPlayerBP (Game|Player|GetPlayerPawn 0)))
  (Variables|Default|SetPlayerBP _asother_player_bp))

(fn ConstructionScript)

(fn OnPickUp
  (params (PickUpType :type BP%20Pick%20Up%20Base%20Object%20Reference))
  (Utilities|Casting|CastToBPPickUpMashroom PickUpType
    (:then
      (Default|ScaleControl (Variables|Default|GetPlayerBP) true)
      (Development|PrintString "Mushroom!" true true "(R=1.000000,G=0.093690,B=0.103637,A=1.000000)"))
    (:CastFailed
      (Utilities|Casting|CastToBPPickUpRing PickUpType)
      (Variables|Default|SetRingsCollected (+ (Variables|Default|GetRingsCollected) 1))
      (Development|PrintString "$$$$$!" true true "(R=1.000000,G=0.927876,B=0.231069,A=1.000000)"))))