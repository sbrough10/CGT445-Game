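; ProjectileBP is a projectile actor that reacts to bricks and goblins it overlaps, scaled to three times size on construction.
; Its sphere overlap runs a sequence of casts, calling Impact on BP_brick or Damage with type-specific amounts on BP_brick1 and BPGoblin, then destroys itself.
; A Hit event also destroys the actor after a one-second delay.
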(event OnComponentBeginOverlap(Sphere)
  (params (OverlappedComponent :type Primitive%20Component%20Object%20Reference) (OtherActor :type Actor%20Object%20Reference) (OtherComp :type Primitive%20Component%20Object%20Reference) (OtherBodyIndex :type Integer) (bFromSweep :type Boolean) (SweepResult :type Hit%20Result%20Structure%20%28by%20ref%29))
  (Utilities|FlowControl|Sequence
    (:then_0
      (bind _asbp_brick (Utilities|Casting|CastToBP_brick OtherActor))
      (Default|Impact _asbp_brick)
      (Actor|DestroyActor))
    (:then_1
      (bind _asbp_brick_1 (Utilities|Casting|CastToBP_brick1 OtherActor))
      (Default|Damage _asbp_brick_1 25)
      (Actor|DestroyActor))
    (:then_2
      (bind _asbpgoblin (Utilities|Casting|CastToBPGoblin OtherActor))
      (Default|Damage _asbpgoblin 50)
      (Actor|DestroyActor))))

(event Collision|EventHit
  (params (MyComp :type Primitive%20Component%20Object%20Reference) (Other :type Actor%20Object%20Reference) (OtherComp :type Primitive%20Component%20Object%20Reference) (bSelfMoved :type Boolean) (HitLocation :type Vector :default "0, 0, 0") (HitNormal :type Vector :default "0, 0, 0") (NormalImpulse :type Vector :default "0, 0, 0") (Hit :type Hit%20Result%20Structure%20%28by%20ref%29))
  (Utilities|FlowControl|Delay 1.0)
  (Actor|DestroyActor))

(fn ConstructionScript
  (Transformation|SetActorScale3D "3.000000,3.000000,3.000000"))