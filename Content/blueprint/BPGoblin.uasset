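; BPGoblin is a Paper2D goblin enemy that hurts the player on contact.
; Its capsule overlap applies damage to otherPlayerBP actors, while its Damage event reduces EnemyHealth and destroys the goblin at zero or below.
; The construction script snaps it to the Y=0 plane.
; An unconnected Timeline holds patrol logic that lerps between PointA and PointB and flips the flipbook, but never runs.
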(event OnComponentBeginOverlap(Capsule)
  (params (OverlappedComponent :type Primitive%20Component%20Object%20Reference) (OtherActor :type Actor%20Object%20Reference) (OtherComp :type Primitive%20Component%20Object%20Reference) (OtherBodyIndex :type Integer) (bFromSweep :type Boolean) (SweepResult :type Hit%20Result%20Structure%20%28by%20ref%29))
  (bind _asother_player_bp (Utilities|Casting|CastTootherPlayerBP OtherActor))
  (bind _output_get (Variables|Default|SetPlayerBP _asother_player_bp))
  (Game|Damage|ApplyDamage _output_get 1e+01 0 0))

(event Custom|Damage
  (params (DamageInt :type Integer))
  ;[1 1 1] take damage
  (bind _output_get (Variables|Default|SetEnemyHealth (- (Variables|Default|GetEnemyHealth) DamageInt)))
  (if (<= _output_get 0)
    (Actor|DestroyActor)))

(fn ConstructionScript
  (bind _returnvalue (Transformation|GetActorLocation))
  (Transformation|SetActorLocation (Math|Vector|MakeVector (.x _returnvalue) 0.0 (.z _returnvalue)) false false))